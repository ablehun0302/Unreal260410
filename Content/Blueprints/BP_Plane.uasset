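; BP_Plane is a player-controlled plane pawn that constantly flies along its forward vector using FloatingPawnMovement.
; Pitch and Roll axes rotate it locally, scaled by rotation speed and delta time, so steering changes its flight direction.
; Fire spawns a BP_Rocket at the launch point.
; Booster plays a timeline that lerps the movement's max speed between default and boost values.
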(event EventTick
  (params (DeltaSeconds :type Float%20%28single-precision%29))
  ;[0.15 0.15 0.15 0.5] 앞으로 움직이기
  (Pawn|Input|AddMovementInput (Transformation|GetActorForwardVector) 1.0 false))

(event Input|ActionEvents|InputActionFire
  (params (Key :type Key%20Structure :default "None"))
  ;[0.15 0.15 0.15 0.5] 미사일 쏘기
  (:Pressed
    (Game|SpawnActorfromClass "/Game/Blueprints/BP_Rocket.BP_Rocket_C" (Transformation|GetWorldTransform (Variables|Default|GetRocketLaunchPoint)) "Undefined" "MultiplyWithRoot" 0 0)))

(event Input|ActionEvents|InputActionBooster
  (params (Key :type Key%20Structure :default "None"))
  ;[0.15 0.15 0.15 0.5] 부스터
  (:Pressed
    (bind _alpha (Timeline|Timeline PlayFromStart)
      (:Update
        (Variables|/Script/Engine.FloatingPawnMovement|SetMaxSpeed (Variables|Default|GetFloatingPawnMovement) (Math|Float|Lerp (Variables|Default|GetDefaultMoveSpeed) (Variables|Default|GetBoosterMoveSpeed) _alpha))))))

(event Input|AxisEvents|InputAxisPitch
  (params (AxisValue :type Float%20%28single-precision%29))
  ;[0.15 0.15 0.15 0.5] 피치 롤 조정
  (Transformation|AddActorLocalRotation (Math|Rotator|MakeRotator 0.0 (* AxisValue (Variables|Default|GetRotationSpeed) (Utilities|Time|GetWorldDeltaSeconds)) 0.0) false false))

(event Input|AxisEvents|InputAxisRoll
  (params (AxisValue :type Float%20%28single-precision%29))
  ;[0.15 0.15 0.15 0.5] 피치 롤 조정
  (Transformation|AddActorLocalRotation (Math|Rotator|MakeRotator (* AxisValue (Variables|Default|GetRotationSpeed) (Utilities|Time|GetWorldDeltaSeconds)) 0.0 0.0) false false))

(fn ConstructionScript)